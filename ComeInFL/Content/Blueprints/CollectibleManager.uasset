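; CollectibleManager counts the items collected in the game and reports the total to the rover's HUD.
; Initalize stores the RoverHUD reference, and Collect passes a collectible to AddToInventory before destroying its actor.
; AddToInventory increments a simple Inventory counter, without storing the item, and pushes the new count to the HUD.
; A debug function that prints the count exists but is left unconnected.
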(event `Initalize`
  (params (`Rover HUD` :type "/Game/Blueprints/RoverHUD Object Reference"))
  (set `self.RoverHUD` `Rover HUD`))

(event `self.ReceiveTick`
  (params (DeltaSeconds :type "Float (single-precision)")))

(event `Collect`
  (params (Collectible :type "/Game/Blueprints/Collectible Object Reference"))
  (`self.Add to Inventory` Collectible)
  (`Actor.K2_DestroyActor` Collectible))

(fn `Add to Inventory`
  (params (`New item` :type "/Game/Blueprints/Collectible Object Reference"))
  (bind _result (`/Engine/EditorBlueprintResources/StandardMacros.IncrementInt` (`self.Inventory`))
    (:`  `
      (`/Game/Blueprints/RoverHUD.SetInventoryCount` (`self.RoverHUD`) _result))))

(fn `DebugPrintInventory`
  (`KismetSystemLibrary.PrintString` (`KismetStringLibrary.Concat_StrStr` "Inventory: " (`KismetStringLibrary.Conv_IntToString` (`self.Inventory`))) true true (struct :`G` 0.66 :`B` 1.0 :`A` 1.0) 0.0))